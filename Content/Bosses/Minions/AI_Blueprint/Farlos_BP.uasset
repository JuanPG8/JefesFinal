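; Farlos_BP is a boss minion character that attacks with a scythe and dies when its health runs out.
; On BeginPlay it spawns Guadaña_BP and attaches it to a mesh socket.
; HacerAtaque starts the attack montage or, if already active, checks its section to queue the second attack.
; AnyDamage reduces Salud; at zero, movement stops and the death montage plays before scythe and minion are destroyed.
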(event Custom|HacerAtaque
  (bind _mesh (Variables|Character|GetMesh))
  (bind _returnvalue (Components|SkeletalMesh|GetAnimInstance _mesh))
  (bind _returnvalue_2 (Animation|Montage|MontageGetCurrentSection _returnvalue "/Game/Bosses/Minions/Animaciones/Ataque_MinionsMontage.Ataque_MinionsMontage"))
  (if (Class|AnimInstance|MontageIsActive _returnvalue "/Game/Bosses/Minions/Animaciones/Ataque_MinionsMontage.Ataque_MinionsMontage")
    (switch name _returnvalue_2
      (:Ataque1
        (Class|AnimInstance|MontageSetNextSection _returnvalue _returnvalue_2 "Ataque2" "/Game/Bosses/Minions/Animaciones/Ataque_MinionsMontage.Ataque_MinionsMontage")))
    (else
      (Animation|PlayAnimMontage "/Game/Bosses/Minions/Animaciones/Ataque_MinionsMontage.Ataque_MinionsMontage" 1.0 "Ataque1"))))

(event Custom|CrearEspada
  (bind _returnvalue (Game|SpawnActorfromClass "/Game/Bosses/Minions/AI_Blueprint/Guadaña_BP.Guadaña_BP_C" (Transformation|GetActorTransform) "Undefined" 0 0))
  (Transformation|AttachComponentToComponent _returnvalue (Variables|Character|GetMesh) "Guadaña" "SnapToTarget" "SnapToTarget" "SnapToTarget" true)
  (Variables|Default|SetGuadana _returnvalue))

(event EventBeginPlay
  (CallFunction|CrearEspada))

(event Collision|EventActorBeginOverlap
  (params (OtherActor :type Actor%20Object%20Reference)))

(event EventTick
  (params (DeltaSeconds :type Float%20%28single-precision%29)))

(event Game|Damage|EventAnyDamage
  (params (Damage :type Float%20%28single-precision%29) (DamageType :type Damage%20Type%20Object%20Reference) (InstigatedBy :type Controller%20Object%20Reference) (DamageCauser :type Actor%20Object%20Reference))
  (bind _output_get (Variables|Default|SetSalud (- (Variables|Default|GetSalud) Damage)))
  (if (<= _output_get 0.0)
    (Utilities|FlowControl|DoOnce false
      (:Completed
        (Pawn|Components|CharacterMovement|DisableMovement (Variables|Character|GetCharacterMovement))
        (bind _returnvalue (Animation|PlayAnimMontage "/Game/Bosses/Minions/Animaciones/Muerte_Montage.Muerte_Montage" 1.0 ""))
        (Utilities|FlowControl|Delay _returnvalue)
        (Actor|DestroyActor (Variables|Default|GetGuadana))
        (Actor|DestroyActor)))))

(fn ConstructionScript)